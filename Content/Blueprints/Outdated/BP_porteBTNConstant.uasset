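; An outdated door wall actor, apparently meant for a constant button, that shifts vertically when its custom events are called.
; MoveBlockConstant raises the actor by BlockDistance from the MurPorte component's current world location, using a swept transform.
; ResetBlock lowers it by the same distance with sweep and teleport enabled.
; Both moves are instant and relative to the current position, with no timeline or stored start point.
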(event `MoveBlockConstant`
  (bind (_returnvalue_x _returnvalue_y _returnvalue_z) (`KismetMathLibrary.BreakVector` (`SceneComponent.K2_GetComponentLocation` (`self.MurPorte`))))
  (`self.K2_SetActorTransform` (`KismetMathLibrary.MakeTransform` (`KismetMathLibrary.MakeVector` _returnvalue_x _returnvalue_y (+ _returnvalue_z (`self.BlockDistance`)))) true))

(event `ResetBlock`
  (bind (_returnvalue_x _returnvalue_y _returnvalue_z) (`KismetMathLibrary.BreakVector` (`SceneComponent.K2_GetComponentLocation` (`self.MurPorte`))))
  (`self.K2_SetActorTransform` (`KismetMathLibrary.MakeTransform` (`KismetMathLibrary.MakeVector` _returnvalue_x _returnvalue_y (- _returnvalue_z (`self.BlockDistance`)))) true true))

(fn `UserConstructionScript`)