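; Outdated text display actor that shows a French prompt built from text components and two sets of four directional logo planes, solid and ghost.
; Custom events toggle visibility: Txt01_on reveals the texts and both logos, but nothing here calls it, and logo02_off is empty.
; The box trigger only prints debug in/out for the main character, hiding the first text on exit.
; Construction refreshes a shadowless widget component.
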(event `self.ReceiveBeginPlay`)

(event `self.Box.OnComponentBeginOverlap`
  (params (OverlappedComponent :type "PrimitiveComponent Object Reference") (OtherActor :type "Actor Object Reference") (OtherComp :type "PrimitiveComponent Object Reference") (OtherBodyIndex :type Integer) (bFromSweep :type Boolean) (SweepResult :type "HitResult Structure (by ref)"))
  (cast `/Game/Blueprints/Character/BP_MainThirdPersonCharacter` OtherActor)
  (`KismetSystemLibrary.PrintString` "in" true true (struct :`R` 1.0 :`G` 0.151328 :`B` 0.091597 :`A` 1.0) 1.0))

(event `self.Box.OnComponentEndOverlap`
  (params (OverlappedComponent :type "PrimitiveComponent Object Reference") (OtherActor :type "Actor Object Reference") (OtherComp :type "PrimitiveComponent Object Reference") (OtherBodyIndex :type Integer))
  (cast `/Game/Blueprints/Character/BP_MainThirdPersonCharacter` OtherActor)
  (`KismetSystemLibrary.PrintString` "out" true true (struct :`R` 1.0 :`G` 0.432794 :`B` 0.851164 :`A` 1.0) 1.0)
  (`SceneComponent.SetVisibility` (`self.TxT1_1_appuyer`) false false))

(event `Txt01_on`
  (`|ExecutionSequence`
    (:`then_0`
      (`SceneComponent.SetVisibility` (`self.TxT1_1_appuyer`) true false))
    (:`then_1`
      (`self.logo01`))
    (:`then_2`
      (`SceneComponent.SetVisibility` (`self.txt1_2_pour`) true false))
    (:`then_3`
      (`SceneComponent.SetVisibility` (`self.txt1_3_represente`) true false))
    (:`then_4`
      (`self.logo02`))))

(event `logo01_0ff`
  (`|ExecutionSequence`
    (:`then_0`
      (`SceneComponent.SetVisibility` (`self.plane_left`) false false))
    (:`then_1`
      (`SceneComponent.SetVisibility` (`self.plane_down`) false false))
    (:`then_2`
      (`SceneComponent.SetVisibility` (`self.plane_right`) false false))
    (:`then_3`
      (`SceneComponent.SetVisibility` (`self.plane_up`) false false))))

(event `logo01`
  (`|ExecutionSequence`
    (:`then_0`
      (`SceneComponent.SetVisibility` (`self.plane_left`) true false))
    (:`then_1`
      (`SceneComponent.SetVisibility` (`self.plane_down`) true false))
    (:`then_2`
      (`SceneComponent.SetVisibility` (`self.plane_right`) true false))
    (:`then_3`
      (`SceneComponent.SetVisibility` (`self.plane_up`) true false))))

(event `logo02`
  (`|ExecutionSequence`
    (:`then_0`
      (`SceneComponent.SetVisibility` (`self.plane_ghost_left`) true false))
    (:`then_1`
      (`SceneComponent.SetVisibility` (`self.plane_ghoest_down`) true false))
    (:`then_2`
      (`SceneComponent.SetVisibility` (`self.plane_ghost_right`) true false))
    (:`then_3`
      (`SceneComponent.SetVisibility` (`self.plane_ghoest_up`) true false))))

(event `logo02_off`)

(fn `UserConstructionScript`
  (bind _bpc_widget (`self.BPC_Widget`))
  (`PrimitiveComponent.SetCastShadow` _bpc_widget false)
  (`/Game/Blueprints/Components/BPC_Widget.UpdateWidget` _bpc_widget))