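; GameStateAxis is a Blueprint, apparently a game state, meant to auto-hide the mouse cursor when idle.
; Disconnected logic compares stored axis values with current input, showing the cursor and clearing the timer on change.
; When unchanged, a resettable DoOnce starts a short timer to HideCursor, which hides the cursor and stores the axes.
; Tick is empty, so the detection never runs.
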(event `ResetHide`
  (`/Engine/EditorBlueprintResources/StandardMacros.DoOnce` false :!via `Reset`
    (:`Completed`
      (set `self.Is mouse moving` false)
      (bind _returnvalue (`KismetSystemLibrary.K2_SetTimerDelegate` (delegate `HideCursor`) 1.5))
      (bind _output_get (set `self.ShowCursorTimer` _returnvalue)))))

(event `HideCursor`
  (set `PlayerController.bShowMouseCursor` false (`GameplayStatics.GetPlayerController` 0))
  (set `self.Mouse Pos X` (`self.GetInputAxisKeyValue`))
  (set `self.Mouse Pos Y` (`self.GetInputAxisKeyValue`)))

(event `self.ReceiveTick`
  (params (DeltaSeconds :type "Float (single-precision)")))

(fn `UserConstructionScript`)