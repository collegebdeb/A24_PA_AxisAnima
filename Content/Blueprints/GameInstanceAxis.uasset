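; Game instance that keeps a death counter (Mort) and shows level hint widgets based on it.
; MortScore adds a full point to the counter and ReloadScore adds half a point.
; IndiceScore2 to IndiceScore4 map the counter to one of three hint tiers in NiveauIndice, print it, then add that level's IndiceLevel widget to the viewport.
; Below the lowest threshold, no hint appears.
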(event `ReloadScore`
  (set `self.mort` (+ (`self.mort`) 0.5)))

(event `MortScore`
  (set `self.mort` (+ (`self.mort`) 1.0)))

(event `IndiceScore2`
  (bind _mort (`self.mort`))
  (bind _mort_2 (`self.mort`))
  (`|ExecutionSequence`
    (:`then_0`
      (if (>= _mort 3.0)
        (if (< _mort 6.0)
          (bind _output_get (set `self.niveauIndice` 1.0))
          (`KismetSystemLibrary.PrintString` (`KismetStringLibrary.Conv_DoubleToString` _output_get))
          (bind _returnvalue (`|CreateWidget` "/Game/UI_Widgets/UI_aideLevel/IndiceLevel02.IndiceLevel02_C" :!label _label))
          (`UserWidget.AddToViewport` _returnvalue 0))))
    (:`then_1`
      (if (>= _mort_2 6.0)
        (if (< _mort_2 10.0)
          (bind _output_get_2 (set `self.niveauIndice` 2.0))
          (`KismetSystemLibrary.PrintString` (`KismetStringLibrary.Conv_DoubleToString` _output_get_2))
          (goto _label))))
    (:`then_2`
      (if (>= (`self.mort`) 10.0)
        (bind _output_get_3 (set `self.niveauIndice` 3.0))
        (`KismetSystemLibrary.PrintString` (`KismetStringLibrary.Conv_DoubleToString` _output_get_3))
        (goto _label)))))

(event `IndiceScore3`
  (bind _mort (`self.mort`))
  (bind _mort_2 (`self.mort`))
  (`|ExecutionSequence`
    (:`then_0`
      (if (>= _mort 3.0)
        (if (< _mort 6.0)
          (bind _output_get (set `self.niveauIndice` 1.0))
          (`KismetSystemLibrary.PrintString` (`KismetStringLibrary.Conv_DoubleToString` _output_get))
          (bind _returnvalue (`|CreateWidget` "/Game/UI_Widgets/UI_aideLevel/IndiceLevel03.IndiceLevel03_C" :!label _label_2))
          (`UserWidget.AddToViewport` _returnvalue 0))))
    (:`then_1`
      (if (>= _mort_2 6.0)
        (if (< _mort_2 10.0)
          (bind _output_get_2 (set `self.niveauIndice` 2.0))
          (`KismetSystemLibrary.PrintString` (`KismetStringLibrary.Conv_DoubleToString` _output_get_2))
          (goto _label_2))))
    (:`then_2`
      (if (>= (`self.mort`) 10.0)
        (bind _output_get_3 (set `self.niveauIndice` 3.0))
        (`KismetSystemLibrary.PrintString` (`KismetStringLibrary.Conv_DoubleToString` _output_get_3))
        (goto _label_2)))))

(event `IndiceScore4`
  (bind _mort (`self.mort`))
  (bind _mort_2 (`self.mort`))
  (`|ExecutionSequence`
    (:`then_0`
      (if (>= _mort 3.0)
        (if (< _mort 6.0)
          (bind _output_get (set `self.niveauIndice` 1.0))
          (`KismetSystemLibrary.PrintString` (`KismetStringLibrary.Conv_DoubleToString` _output_get))
          (bind _returnvalue (`|CreateWidget` "/Game/UI_Widgets/UI_aideLevel/IndiceLevel04.IndiceLevel04_C" :!label _label_3))
          (`UserWidget.AddToViewport` _returnvalue 0))))
    (:`then_1`
      (if (>= _mort_2 6.0)
        (if (< _mort_2 10.0)
          (bind _output_get_2 (set `self.niveauIndice` 2.0))
          (`KismetSystemLibrary.PrintString` (`KismetStringLibrary.Conv_DoubleToString` _output_get_2))
          (goto _label_3))))
    (:`then_2`
      (if (>= (`self.mort`) 10.0)
        (bind _output_get_3 (set `self.niveauIndice` 3.0))
        (`KismetSystemLibrary.PrintString` (`KismetStringLibrary.Conv_DoubleToString` _output_get_3))
        (goto _label_3)))))