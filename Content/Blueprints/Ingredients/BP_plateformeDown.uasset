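; BP_plateformeDown is a platform that the player character can pass through by crouching.
; A Box overlap tracks when BP_MainThirdPersonCharacter is in range and stores a reference to it.
; While it overlaps, Tick sets the platform's Pawn collision response to Ignore if the character crouches, otherwise to Block.
; Ending the overlap only clears the flag, so the last collision response persists.
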(event `self.ReceiveTick`
  (params (DeltaSeconds :type "Float (single-precision)"))
  (bind _plateforme (`self.Plateforme`))
  (if (`self.IsOverlapPlayer`)
    (if (`/Game/Blueprints/Character/BP_MainThirdPersonCharacter.Is crouch` (stale `self.Box.OnComponentBeginOverlap` _asbp_main_third_person_character))
      (`PrimitiveComponent.SetCollisionResponseToChannel` _plateforme "ECC_Pawn" "ECR_Ignore")
      (else
        (`PrimitiveComponent.SetCollisionResponseToChannel` _plateforme "ECC_Pawn" "ECR_Block")))))

(event `self.Box.OnComponentBeginOverlap`
  (params (OverlappedComponent :type "PrimitiveComponent Object Reference") (OtherActor :type "Actor Object Reference") (OtherComp :type "PrimitiveComponent Object Reference") (OtherBodyIndex :type Integer) (bFromSweep :type Boolean) (SweepResult :type "HitResult Structure (by ref)"))
  (bind _asbp_main_third_person_character (cast `/Game/Blueprints/Character/BP_MainThirdPersonCharacter` OtherActor))
  (set `self.IsOverlapPlayer` true))

(event `self.Box.OnComponentEndOverlap`
  (params (OverlappedComponent :type "PrimitiveComponent Object Reference") (OtherActor :type "Actor Object Reference") (OtherComp :type "PrimitiveComponent Object Reference") (OtherBodyIndex :type Integer))
  (cast `/Game/Blueprints/Character/BP_MainThirdPersonCharacter` OtherActor)
  (set `self.IsOverlapPlayer` false))

(fn `UserConstructionScript`)