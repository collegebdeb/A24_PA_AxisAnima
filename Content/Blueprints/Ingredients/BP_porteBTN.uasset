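; BP_porteBTN is a door or pillar actor that slides away when its OpenSesame event fires, presumably from a button.
; OpenSesame caches the root's world location, then branches on DirectionsPilier to move by a BlockDistance-based offset.
; Up and Right animate through timelines, with Up re-caching position when finished, while Down and Left jump in one step.
; MovePilier adds the offset to the cached position and sets the root's relative location with sweep.
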(event `OpenSesame`
  (bind _blockdistance (`self.BlockDistance`))
  (`self.SetPosition`)
  (switch `/Game/Blueprints/Enums/E_Directions` (`self.DirectionsPilier`)
    (:`NewEnumerator0`
      (bind (_direction _newtrack_0) (`Timeline|TimelineLiftAnimation` :!via `PlayFromStart`)
        (:`Update`
          (`self.MovePilier` 0.0 0.0 (* _newtrack_0 _blockdistance)))
        (:`Finished`
          (`self.SetPosition`))))
    (:`NewEnumerator3`
      (bind (_direction_2 _float_multiplier) (`Timeline|Timeline` :!via `PlayFromStart`)
        (:`Update`
          (`self.MovePilier` 0.0 (* _float_multiplier _blockdistance)))))
    (:`NewEnumerator1`
      (bind _result (`/Engine/EditorBlueprintResources/StandardMacros.NegateFloat` _blockdistance)
        (:`  `
          (`self.MovePilier` 0.0 0.0 _result))))
    (:`NewEnumerator2`
      (bind _result_2 (`/Engine/EditorBlueprintResources/StandardMacros.NegateFloat` _blockdistance)
        (:`  `
          (`self.MovePilier` 0.0 _result_2))))))

(event `SetPosition`
  (bind (_returnvalue_x _returnvalue_y _returnvalue_z) (`KismetMathLibrary.BreakVector` (`SceneComponent.K2_GetComponentLocation` (`self.DefaultSceneRoot`))))
  (set `self.Val_X` _returnvalue_x)
  (set `self.Val_Y` _returnvalue_y)
  (set `self.Val_Z` _returnvalue_z))

(fn `MovePilier`
  (params (Val_Move_X :type "Float (double-precision)") (Val_Move_Y :type "Float (double-precision)") (Val_Move_Z :type "Float (double-precision)"))
  (if true
    (`SceneComponent.K2_SetRelativeLocation` (`self.DefaultSceneRoot`) (`KismetMathLibrary.MakeVector` (+ (`self.Val_X`) Val_Move_X) (+ (`self.Val_Y`) Val_Move_Y) (+ (`self.Val_Z`) Val_Move_Z)) true false)
    (return)))

(fn `UserConstructionScript`)