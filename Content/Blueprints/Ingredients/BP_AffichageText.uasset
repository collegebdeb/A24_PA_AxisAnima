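; BP_AffichageText is a proximity text display actor that shows a widget while the main third-person character stands inside its box trigger.
; The widget component starts hidden on BeginPlay, then box begin and end overlap events toggle its visibility, including children, for that character class only.
; The construction script disables the widget's shadow casting and refreshes it.
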(event `self.ReceiveBeginPlay`
  (`SceneComponent.SetVisibility` (`self.BPC_Widget`) false true))

(event `self.Box.OnComponentBeginOverlap`
  (params (OverlappedComponent :type "PrimitiveComponent Object Reference") (OtherActor :type "Actor Object Reference") (OtherComp :type "PrimitiveComponent Object Reference") (OtherBodyIndex :type Integer) (bFromSweep :type Boolean) (SweepResult :type "HitResult Structure (by ref)"))
  (cast `/Game/Blueprints/Character/BP_MainThirdPersonCharacter` OtherActor)
  (`SceneComponent.SetVisibility` (`self.BPC_Widget`) true true))

(event `self.Box.OnComponentEndOverlap`
  (params (OverlappedComponent :type "PrimitiveComponent Object Reference") (OtherActor :type "Actor Object Reference") (OtherComp :type "PrimitiveComponent Object Reference") (OtherBodyIndex :type Integer))
  (cast `/Game/Blueprints/Character/BP_MainThirdPersonCharacter` OtherActor)
  (`SceneComponent.SetVisibility` (`self.BPC_Widget`) false true))

(fn `UserConstructionScript`
  (bind _bpc_widget (`self.BPC_Widget`))
  (`PrimitiveComponent.SetCastShadow` _bpc_widget false)
  (`/Game/Blueprints/Components/BPC_Widget.UpdateWidget` _bpc_widget))