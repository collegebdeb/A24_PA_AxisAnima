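; BP_BlocPossedable is a clickable block that the player possesses to set it moving in the direction currently selected on BP_MainThirdPersonCharacter.
; On click, if BPCMouvementBloc allows possession, it maps DirectionMouvement to the component's direction, blocks that move on the character and recolors the block.
; It then starts the component's movement and resets the character's values; non-possessible blocks only trigger the reset.
; Only the up case also applies the highlight overlay.
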(event `self.ReceiveBeginPlay`
  (add `self.OnClicked` (delegate `PossessionClick`)))

(event `self.ReceiveTick`
  (params (DeltaSeconds :type "Float (single-precision)")))

(event `PossessionClick` :!signature `self.OnClicked`
  (params (TouchedActor :type "Actor Object Reference") (ButtonPressed :type "Key Structure" :default "None"))
  (bind _bpc_mouvementbloc (`self.BPC_MouvementBloc`))
  (bind `_bloc_possédable` (`self.Bloc_Possédable`))
  (bind _returnvalue (`GameplayStatics.GetActorOfClass` "/Game/Blueprints/Character/BP_MainThirdPersonCharacter.BP_MainThirdPersonCharacter_C"))
  (bind _asbp_main_third_person_character (cast `/Game/Blueprints/Character/BP_MainThirdPersonCharacter` _returnvalue))
  (if (`/Game/Blueprints/Components/BPC_MouvementBloc.IsPossessible` _bpc_mouvementbloc)
    (switch `int` (`/Game/Blueprints/Character/BP_MainThirdPersonCharacter.DirectionMouvement` _asbp_main_third_person_character)
      (:`1`
        (set `/Game/Blueprints/Components/BPC_MouvementBloc.Directions` "NewEnumerator0" _bpc_mouvementbloc)
        (set `/Game/Blueprints/Character/BP_MainThirdPersonCharacter.CantMoveUp` true _asbp_main_third_person_character)
        (`PrimitiveComponent.SetMaterial` `_bloc_possédable` 0 "/Game/Art/Materiaux/MI_couleurHaut.MI_couleurHaut")
        (`MeshComponent.SetOverlayMaterial` `_bloc_possédable` "/Game/Art/PostProcess_Materials/MI_Highlight.MI_Highlight"))
      (:`2`
        (set `/Game/Blueprints/Components/BPC_MouvementBloc.Directions` "NewEnumerator2" _bpc_mouvementbloc)
        (set `/Game/Blueprints/Character/BP_MainThirdPersonCharacter.CantMoveLeft` true _asbp_main_third_person_character)
        (`PrimitiveComponent.SetMaterial` `_bloc_possédable` 0 "/Game/Art/Materiaux/MI_couleurArriere.MI_couleurArriere"))
      (:`3`
        (set `/Game/Blueprints/Components/BPC_MouvementBloc.Directions` "NewEnumerator1" _bpc_mouvementbloc)
        (set `/Game/Blueprints/Character/BP_MainThirdPersonCharacter.CantMoveDown` true _asbp_main_third_person_character)
        (`PrimitiveComponent.SetMaterial` `_bloc_possédable` 0 "/Game/Art/Materiaux/MI_couleurBas.MI_couleurBas"))
      (:`4`
        (set `/Game/Blueprints/Components/BPC_MouvementBloc.Directions` "NewEnumerator3" _bpc_mouvementbloc)
        (set `/Game/Blueprints/Character/BP_MainThirdPersonCharacter.CantMoveRight` true _asbp_main_third_person_character)
        (`PrimitiveComponent.SetMaterial` `_bloc_possédable` 0 "/Game/Art/Materiaux/MI_couleurAvant.MI_couleurAvant")))
    (`/Game/Blueprints/Components/BPC_MouvementBloc.StartEventMoving` _bpc_mouvementbloc)
    (`/Game/Blueprints/Character/BP_MainThirdPersonCharacter.ResetValeur` _asbp_main_third_person_character)
    (else
      (`/Game/Blueprints/Character/BP_MainThirdPersonCharacter.ResetValeur` _asbp_main_third_person_character))))

(fn `UserConstructionScript`)