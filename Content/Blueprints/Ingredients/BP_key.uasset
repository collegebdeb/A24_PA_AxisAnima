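; BP_key is a key pickup that spins in place and, when the player character touches it, grants the key and opens the next-level door.
; A looping timeline, played from Tick, drives the key mesh's world yaw.
; On trigger-sphere overlap it sets the character's KeyPass, plays a pickup sound scaled by the game instance's volume setting, then after a short delay calls OpenDoor on BP_prochainNiveau and destroys itself.
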(event `self.ReceiveBeginPlay`)

(event `self.ReceiveTick`
  (params (DeltaSeconds :type "Float (single-precision)"))
  (bind _key (`self.key`))
  (bind (_returnvalue_roll _returnvalue_pitch) (`KismetMathLibrary.BreakRotator` (`SceneComponent.K2_GetComponentRotation` _key)))
  (bind (_direction _alpha) (`Timeline|Timeline` :!label _label)
    (:`Update`
      (`SceneComponent.K2_SetWorldRotation` _key (`KismetMathLibrary.MakeRotator` _returnvalue_roll _returnvalue_pitch (* _alpha 1.0)) false false))
    (:`Finished`
      (goto _label :!via `PlayFromStart`))))

(event `self.KeyTriggerSphere.OnComponentBeginOverlap`
  (params (OverlappedComponent :type "PrimitiveComponent Object Reference") (OtherActor :type "Actor Object Reference") (OtherComp :type "PrimitiveComponent Object Reference") (OtherBodyIndex :type Integer) (bFromSweep :type Boolean) (SweepResult :type "HitResult Structure (by ref)"))
  (bind _asbp_main_third_person_character (cast `/Game/Blueprints/Character/BP_MainThirdPersonCharacter` OtherActor))
  (set `/Game/Blueprints/Character/BP_MainThirdPersonCharacter.KeyPass` 1 _asbp_main_third_person_character)
  (`KismetSystemLibrary.PrintString` "Key 1" true true (struct :`R` 0.155993 :`G` 1.0 :`B` 0.819444 :`A` 1.0))
  (bind _asgame_instance_axis (cast `/Game/Blueprints/GameInstanceAxis` (`GameplayStatics.GetGameInstance`)))
  (`GameplayStatics.PlaySound2D` "/Game/Son/audio/keyGet.keyGet" (/ (`/Game/Blueprints/GameInstanceAxis.SonInstance` _asgame_instance_axis) 100.0) 1.0 0.0 null null)
  (`KismetSystemLibrary.Delay` 0.2)
  (bind _returnvalue (`GameplayStatics.GetActorOfClass` "/Game/Blueprints/Ingredients/BP_prochainNiveau.BP_prochainNiveau_C"))
  (`/Game/Blueprints/Ingredients/BP_prochainNiveau.OpenDoor` _returnvalue)
  (`self.K2_DestroyActor`))

(fn `UserConstructionScript`)