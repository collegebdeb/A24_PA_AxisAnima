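; BP_killbox is a trigger volume that kills the main third-person character on contact.
; The first Box overlap by any actor passes a DoOnce with no reset and, if still overlapping, calls TriggerDeath.
; TriggerDeath checks that the character is alive, plays GutDrop scaled by the game instance's sound setting, and prints a debug string.
; A second DoOnce then limits the character's death event to one call.
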(event `self.Box.OnComponentBeginOverlap`
  (params (OverlappedComponent :type "PrimitiveComponent Object Reference") (OtherActor :type "Actor Object Reference") (OtherComp :type "PrimitiveComponent Object Reference") (OtherBodyIndex :type Integer) (bFromSweep :type Boolean) (SweepResult :type "HitResult Structure (by ref)"))
  (`/Engine/EditorBlueprintResources/StandardMacros.DoOnce` false
    (:`Completed`
      (if (`PrimitiveComponent.IsOverlappingActor` (`self.Box`) OtherActor)
        (`self.TriggerDeath` OtherActor)))))

(event `TriggerDeath`
  (params (actorOverlap :type "Actor Object Reference"))
  (bind _asbp_main_third_person_character (cast `/Game/Blueprints/Character/BP_MainThirdPersonCharacter` actorOverlap))
  (if (`/Game/Blueprints/Character/BP_MainThirdPersonCharacter.IsAlive` _asbp_main_third_person_character)
    (bind _asgame_instance_axis (cast `/Game/Blueprints/GameInstanceAxis` (`GameplayStatics.GetGameInstance`)))
    (`GameplayStatics.PlaySound2D` "/Game/Son/audio/placeholder/gutDrop.gutDrop" (/ (`/Game/Blueprints/GameInstanceAxis.SonInstance` _asgame_instance_axis) 100.0) 1.0 0.0 null null)
    (`KismetSystemLibrary.PrintString` "SonMort" true true (struct :`R` 1.0 :`G` 0.763009 :`A` 1.0))
    (`/Engine/EditorBlueprintResources/StandardMacros.DoOnce` false
      (:`Completed`
        (`/Game/Blueprints/Character/BP_MainThirdPersonCharacter.EventDeathCharacter` _asbp_main_third_person_character)))))

(fn `UserConstructionScript`)