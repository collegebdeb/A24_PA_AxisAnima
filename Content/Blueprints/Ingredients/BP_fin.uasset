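; BP_fin is an end-of-game trigger that quits the game when the player character enters its box.
; Any overlap plays a squeaky door sound at the GameInstanceAxis volume, before the character check.
; If NeedKey is set, the character needs a positive KeyPass or "Need Key" prints; otherwise movement is disabled and the game quits after a short delay.
; A transition widget is created on BeginPlay but never displayed here.
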(event `self.ReceiveBeginPlay`
  (bind _returnvalue (`|CreateWidget` "/Game/UI_Widgets/UI_Transition.UI_Transition_C"))
  (set `self.Widget_Transition` _returnvalue))

(event `self.Box.OnComponentBeginOverlap`
  (params (OverlappedComponent :type "PrimitiveComponent Object Reference") (OtherActor :type "Actor Object Reference") (OtherComp :type "PrimitiveComponent Object Reference") (OtherBodyIndex :type Integer) (bFromSweep :type Boolean) (SweepResult :type "HitResult Structure (by ref)"))
  (bind _asgame_instance_axis (cast `/Game/Blueprints/GameInstanceAxis` (`GameplayStatics.GetGameInstance`)))
  (`GameplayStatics.PlaySound2D` "/Game/Son/audio/SqeakyDoor.SqeakyDoor" (/ (`/Game/Blueprints/GameInstanceAxis.SonInstance` _asgame_instance_axis) 100.0) 1.0 0.0 null null)
  (`KismetSystemLibrary.PrintString` "SonBtnUI" true true (struct :`R` 1.0 :`G` 0.763009 :`A` 1.0))
  (bind _asbp_main_third_person_character (cast `/Game/Blueprints/Character/BP_MainThirdPersonCharacter` OtherActor))
  (if (`self.NeedKey`)
    (if (> (`/Game/Blueprints/Character/BP_MainThirdPersonCharacter.KeyPass` _asbp_main_third_person_character) 0)
      (`CharacterMovementComponent.DisableMovement` (`Character.CharacterMovement` _asbp_main_third_person_character) :!label _label)
      (`KismetSystemLibrary.Delay` 0.3)
      (`KismetSystemLibrary.QuitGame` null "Quit")
      (else
        (`KismetSystemLibrary.PrintString` "Need Key" true true (struct :`R` 1.0 :`G` 0.149544 :`A` 1.0))))
    (else
      (goto _label))))

(fn `UserConstructionScript`)