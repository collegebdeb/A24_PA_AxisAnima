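; BP_porte is a sliding door that moves a set distance up, down, left or right.
; BeginPlay caches the root's world position, and OpenSesame plays the Chronologie timeline, whose multiplier scales BlockDistance along Z or Y according to DirectionsPilier.
; MovePilier applies that offset to the start position as the root's relative location, without sweep.
; ResetBlock reverses the timeline to slide the door back.
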(event `self.ReceiveBeginPlay`
  (`self.SetPosition`))

(event `self.ReceiveTick`
  (params (DeltaSeconds :type "Float (single-precision)")))

(event `SetPosition`
  (set `self.StartPosition` (`SceneComponent.K2_GetComponentLocation` (`self.DefaultSceneRoot`))))

(event `OpenSesame`
  (bind _blockdistance (`self.BlockDistance`))
  (bind _returnvalue (* _blockdistance -1.0))
  (bind (_direction _float_multiplier) (`Timeline|Chronologie` :!label _label)
    (:`Update`
      (switch `/Game/Blueprints/Enums/E_Directions` (`self.DirectionsPilier`)
        (:`NewEnumerator0`
          (`self.MovePilier` 0.0 0.0 (* _float_multiplier _blockdistance)))
        (:`NewEnumerator3`
          (`self.MovePilier` 0.0 (* _float_multiplier _blockdistance)))
        (:`NewEnumerator1`
          (`self.MovePilier` 0.0 0.0 (* _float_multiplier _returnvalue)))
        (:`NewEnumerator2`
          (`self.MovePilier` 0.0 (* _float_multiplier _returnvalue)))))))

(event `ResetBlock`
  (goto _label :!via `Reverse`))

(fn `MovePilier`
  (params (Val_Move_X :type "Float (double-precision)") (Val_Move_Y :type "Float (double-precision)") (Val_Move_Z :type "Float (double-precision)"))
  (bind (_startposition_x _startposition_y _startposition_z) (`KismetMathLibrary.BreakVector` (`self.StartPosition`)))
  (`SceneComponent.K2_SetRelativeLocation` (`self.DefaultSceneRoot`) (`KismetMathLibrary.MakeVector` (+ _startposition_x Val_Move_X) (+ _startposition_y Val_Move_Y) (+ _startposition_z Val_Move_Z)) false false)
  (return))

(fn `UserConstructionScript`)