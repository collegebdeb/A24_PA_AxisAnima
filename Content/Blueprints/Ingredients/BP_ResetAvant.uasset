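; BP_ResetAvant is a trigger actor that lifts the main character's CantMoveRight lock when that character is inside its box.
; Begin and end overlap toggle an Onoff flag, and while it is set Tick re-runs the check through CheckAvant, reusing the overlap's actor.
; When the lock is found set, it clears it, destroys itself and calls ClickAvant on the first UI_game widget.
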(event `self.ReceiveTick`
  (params (DeltaSeconds :type "Float (single-precision)"))
  (if (`self.on/off`)
    (`self.checkAvant`)))

(event `self.Box.OnComponentBeginOverlap`
  (params (OverlappedComponent :type "PrimitiveComponent Object Reference") (OtherActor :type "Actor Object Reference") (OtherComp :type "PrimitiveComponent Object Reference") (OtherBodyIndex :type Integer) (bFromSweep :type Boolean) (SweepResult :type "HitResult Structure (by ref)"))
  (set `self.on/off` true)
  (bind _asbp_main_third_person_character (cast `/Game/Blueprints/Character/BP_MainThirdPersonCharacter` OtherActor :!label _label))
  (if (`/Game/Blueprints/Character/BP_MainThirdPersonCharacter.CantMoveRight` _asbp_main_third_person_character)
    (set `/Game/Blueprints/Character/BP_MainThirdPersonCharacter.CantMoveRight` false _asbp_main_third_person_character)
    (`self.K2_DestroyActor`)
    (bind _foundwidgets (`WidgetBlueprintLibrary.GetAllWidgetsOfClass` "/Game/UI_Widgets/UI_game.UI_game_C"))
    (`/Game/UI_Widgets/UI_game.ClickAvant` (`|GetArrayItem` _foundwidgets))))

(event `checkAvant`
  (goto _label))

(event `self.Box.OnComponentEndOverlap`
  (params (OverlappedComponent :type "PrimitiveComponent Object Reference") (OtherActor :type "Actor Object Reference") (OtherComp :type "PrimitiveComponent Object Reference") (OtherBodyIndex :type Integer))
  (set `self.on/off` false))

(fn `UserConstructionScript`)