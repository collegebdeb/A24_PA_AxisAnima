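; Hold-down button that drives the BP_porteBTNConstant door while the main third-person character stands on it.
; Overlapping its collision turns the button blue and calls MoveBlockConstant on the door found via GetActorOfClass.
; Leaving restores the material and calls ResetBlock.
; Two DoOnce gates re-arm each other so press and release alternate, each printing a debug string.
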(event `self.CollisionBTN.OnComponentBeginOverlap`
  (params (OverlappedComponent :type "PrimitiveComponent Object Reference") (OtherActor :type "Actor Object Reference") (OtherComp :type "PrimitiveComponent Object Reference") (OtherBodyIndex :type Integer) (bFromSweep :type Boolean) (SweepResult :type "HitResult Structure (by ref)"))
  (cast `/Game/Blueprints/Character/BP_MainThirdPersonCharacter` OtherActor)
  (`/Engine/EditorBlueprintResources/StandardMacros.DoOnce` false :!label _label
    (:`Completed`
      (`KismetSystemLibrary.PrintString` "hit" true true (struct :`R` 0.613307 :`G` 1.0 :`B` 0.599263 :`A` 1.0))
      (`PrimitiveComponent.SetMaterial` (`self.BTN`) 0 "/Game/LevelPrototyping/Materials/MI_Solid_Blue.MI_Solid_Blue")
      (bind _returnvalue (`GameplayStatics.GetActorOfClass` "/Game/Blueprints/Ingredients/BP_porteBTNConstant.BP_porteBTNConstant_C"))
      (bind _asbp_porte_btnconstant (cast `/Game/Blueprints/Ingredients/BP_porteBTNConstant` _returnvalue))
      (`/Game/Blueprints/Ingredients/BP_porteBTNConstant.MoveBlockConstant` _asbp_porte_btnconstant)
      (goto _label_2 :!via `Reset`))))

(event `self.CollisionBTN.OnComponentEndOverlap`
  (params (OverlappedComponent :type "PrimitiveComponent Object Reference") (OtherActor :type "Actor Object Reference") (OtherComp :type "PrimitiveComponent Object Reference") (OtherBodyIndex :type Integer))
  (cast `/Game/Blueprints/Character/BP_MainThirdPersonCharacter` OtherActor)
  (`/Engine/EditorBlueprintResources/StandardMacros.DoOnce` true :!label _label_2
    (:`Completed`
      (`KismetSystemLibrary.PrintString` "out" true true (struct :`R` 0.613307 :`G` 1.0 :`B` 0.599263 :`A` 1.0))
      (`PrimitiveComponent.SetMaterial` (`self.BTN`) 0 "/Game/Blueprints/Character/AAAAAAAA_Material.AAAAAAAA_Material")
      (bind _returnvalue (`GameplayStatics.GetActorOfClass` "/Game/Blueprints/Ingredients/BP_porteBTNConstant.BP_porteBTNConstant_C"))
      (bind _asbp_porte_btnconstant (cast `/Game/Blueprints/Ingredients/BP_porteBTNConstant` _returnvalue))
      (`/Game/Blueprints/Ingredients/BP_porteBTNConstant.ResetBlock` _asbp_porte_btnconstant)
      (goto _label :!via `Reset`))))

(fn `UserConstructionScript`)