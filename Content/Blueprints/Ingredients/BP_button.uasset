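; Pressure button actor that opens the linked doors in PortesBTN when the player character overlaps its collision.
; Pressing swaps the button material to blue and calls OpenSesame on each door.
; Without SwitchMode it fires only once; with it, ending the overlap changes the material again and calls ResetBlock on the doors.
; Two DoOnce gates re-arm each other for the open/close cycle, alongside the LevierActif guard.
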(event `self.CollisionBTN.OnComponentBeginOverlap`
  (params (OverlappedComponent :type "PrimitiveComponent Object Reference") (OtherActor :type "Actor Object Reference") (OtherComp :type "PrimitiveComponent Object Reference") (OtherBodyIndex :type Integer) (bFromSweep :type Boolean) (SweepResult :type "HitResult Structure (by ref)"))
  (bind _portes_btn (`self.Portes BTN`))
  (bind _btn (`self.BTN`))
  (if (not (`self.Levier Actif`))
    (cast `/Game/Blueprints/Character/BP_MainThirdPersonCharacter` OtherActor)
    (`/Engine/EditorBlueprintResources/StandardMacros.DoOnce` false :!label _label
      (:`Completed`
        (set `self.Levier Actif` true)
        (`KismetSystemLibrary.PrintString` "open" true true (struct :`R` 0.613307 :`G` 1.0 :`B` 0.599263 :`A` 1.0))
        (`PrimitiveComponent.SetMaterial` _btn 0 "/Game/LevelPrototyping/Materials/MI_Solid_Blue.MI_Solid_Blue")
        (for _array_element _portes_btn
          (`/Game/Blueprints/Ingredients/BP_porteBTN.OpenSesame` _array_element)
          (`KismetSystemLibrary.PrintString` "CanOpen")
          (if (`self.SwitchMode`)
            (set `self.Levier Actif` false)
            (goto _label_2 :!via `Reset`)))))))

(event `self.CollisionBTN.OnComponentEndOverlap`
  (params (OverlappedComponent :type "PrimitiveComponent Object Reference") (OtherActor :type "Actor Object Reference") (OtherComp :type "PrimitiveComponent Object Reference") (OtherBodyIndex :type Integer))
  (if (`self.SwitchMode`)
    (if (not (`self.Levier Actif`))
      (cast `/Game/Blueprints/Character/BP_MainThirdPersonCharacter` OtherActor)
      (`/Engine/EditorBlueprintResources/StandardMacros.DoOnce` true :!label _label_2
        (:`Completed`
          (set `self.Levier Actif` true)
          (`KismetSystemLibrary.PrintString` "close" true true (struct :`R` 0.613307 :`G` 1.0 :`B` 0.599263 :`A` 1.0))
          (`PrimitiveComponent.SetMaterial` (`self.BTN`) 0 "/Game/Blueprints/Character/AAAAAAAA_Material.AAAAAAAA_Material")
          (for _array_element (`self.Portes BTN`)
            (`/Game/Blueprints/Ingredients/BP_porteBTN.ResetBlock` _array_element)
            (`KismetSystemLibrary.PrintString` "CanBeClose")
            (set `self.Levier Actif` false)
            (goto _label :!via `Reset`)))))))

(fn `UserConstructionScript`)