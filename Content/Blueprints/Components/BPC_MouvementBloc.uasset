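; Actor component that slides its owning block in one of four directions on the Y/Z plane until it hits an obstacle.
; Debug key P starts a looping timer that offsets the owner's root by speed and tick delta, with optional sweep.
; Each step fires two parallel line traces ahead, ignoring the player character; either hit stops movement.
; The delayed CheckIfBlocked follow-up after stopping is an empty stub.
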(event Custom|GoMove
  (if (Variables|Default|GetStopMoving)
    (Utilities|Time|PauseTimerbyHandle (stale Input|KeyboardEvents|DebugKeyP _returnvalue))
    (Development|PrintString "It broke" true true "(R=0.278366,G=0.092419,B=1.000000,A=1.000000)")
    (Utilities|Time|SetTimerbyEvent (delegate Custom|CheckIfBlocked) 2.0)
    (else
      (CallFunction|MoveDirection)
      (if (Variables|Default|GetCollision_Hit)
        (Variables|Default|SetStopMoving true)
        (Development|PrintString "Zucka Zucka" true true "(R=0.278366,G=0.092419,B=1.000000,A=1.000000)")))))

(event Custom|CheckIfBlocked)

(event Custom|MoveDirection
  (bind _deltatime (Variables|Default|GetdeltaTime))
  (bind _valmultiply_lt (Variables|Default|GetValMultiply_LT))
  (bind _valmultiply_lt_2 (Variables|Default|GetValMultiply_LT))
  (bind _valmultiply_lt_3 (Variables|Default|GetValMultiply_LT))
  (bind _val_objectspeed (Variables|Default|GetVal_ObjectSpeed))
  (bind _val_objectspeed_2 (Variables|Default|GetVal_ObjectSpeed))
  (bind _valmultiply_lt_4 (Variables|Default|GetValMultiply_LT))
  (bind _returnvalue (* _deltatime -3e+02 _val_objectspeed_2))
  (bind _returnvalue_2 (* _deltatime 3e+02 _val_objectspeed))
  (switch int (Variables|Default|GetInt_Direction)
    (:0
      (CallFunction|MoveObjet 0.0 0.0 _returnvalue_2)
      (CallFunction|DetectionLineTrace (* "0.000000,0.000000,50.000000" _valmultiply_lt) (* "0.000000,40.000000,0.000000" _valmultiply_lt)))
    (:1
      (CallFunction|MoveObjet 0.0 _returnvalue_2 0.0)
      (CallFunction|DetectionLineTrace (* "0.000000,50.000000,0.000000" _valmultiply_lt_3) (* "0.000000,0.000000,40.000000" _valmultiply_lt_3)))
    (:2
      (CallFunction|MoveObjet 0.0 0.0 _returnvalue)
      (CallFunction|DetectionLineTrace (* "0.000000,0.000000,-50.000000" _valmultiply_lt_2) (* "0.000000,40.000000,0.000000" _valmultiply_lt_2)))
    (:3
      (CallFunction|MoveObjet 0.0 _returnvalue 0.0)
      (CallFunction|DetectionLineTrace (* "0.000000,-50.000000,0.000000" _valmultiply_lt_4) (* "0.000000,0.000000,40.000000" _valmultiply_lt_4)))))

(event EventBeginPlay
  (bind _returnvalue (Actor|GetActorOfClass "/Game/Blueprints/Character/BP_MainThirdPersonCharacter.BP_MainThirdPersonCharacter_C"))
  (Variables|Default|SetActors%20to%20Ignore (Utilities|Array|MakeArray _returnvalue)))

(event EventTick
  (params (DeltaSeconds :type Float%20%28single-precision%29))
  (Variables|Default|SetdeltaTime DeltaSeconds))

(event Input|KeyboardEvents|DebugKeyP
  (params (Key :type Key%20Structure :default "None") (ActionValue :type Input%20Action%20Value%20Structure))
  (:Pressed
    (bind _returnvalue (Utilities|Time|SetTimerbyEvent (delegate Custom|GoMove) (stale EventTick DeltaSeconds) true))))

(fn VecteurBloc
  (bind _self self)
  (bind _returnvalue (Components|GetOwner _self))
  (bind _rootcomponent (Variables|/Script/Engine.Actor|GetRootComponent _returnvalue))
  (return (Transformation|GetWorldLocation _rootcomponent) _rootcomponent))

(fn MoveObjet
  (params (Val_Move-X :type Float%20%28double-precision%29) (Val_Move-Y :type Float%20%28double-precision%29) (Val_Move-Z :type Float%20%28double-precision%29))
  (bind (_vector_owner _root) (CallFunction|VecteurBloc))
  (Transformation|SetRelativeLocation _root (Math|Vector|MakeVector (+ Val_Move-X (.X (Math|Vector|BreakVector _vector_owner))) (+ Val_Move-Y (.Y (Math|Vector|BreakVector _vector_owner))) (+ Val_Move-Z (.Z (Math|Vector|BreakVector _vector_owner)))) (Variables|Default|GetCollisionDetectionOn) false)
  (return))

(fn DetectionLineTrace
  (params (Vector_LT_End :type Vector) (VectorAdd_Position :type Vector))
  (bind _vector_owner (CallFunction|VecteurBloc))
  (Utilities|FlowControl|Sequence
    (:then_0
      (bind _outhit (Collision|LineTraceByChannel (+ _vector_owner VectorAdd_Position) (+ (+ _vector_owner VectorAdd_Position) Vector_LT_End) "TraceTypeQuery2" false (Variables|Default|GetActors%20to%20Ignore) "ForOneFrame" true "(R=1.000000,G=0.000000,B=0.000000,A=1.000000)" "(R=0.000000,G=1.000000,B=0.000000,A=1.000000)" 0.1)))
    (:then_1
      (bind _outhit_2 (Collision|LineTraceByChannel (- _vector_owner VectorAdd_Position) (+ (- _vector_owner VectorAdd_Position) Vector_LT_End) "TraceTypeQuery2" false (Variables|Default|GetActors%20to%20Ignore) "ForOneFrame" true "(R=1.000000,G=0.000000,B=0.000000,A=1.000000)" "(R=0.000000,G=1.000000,B=0.000000,A=1.000000)" 0.1))
      (Variables|Default|SetCollision_Hit (or (.bBlockingHit (Collision|BreakHitResult _outhit)) (.bBlockingHit (Collision|BreakHitResult _outhit_2)))))))