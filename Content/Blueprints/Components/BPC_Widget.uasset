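; Widget component that displays configurable in-game text through a WB_TexteInGame widget.
; On BeginPlay it casts its widget and applies the text, size and color variables to TextBlock1, keeping the other font settings it passes through.
; UpdateWidget waits one tick, then reruns the same setup to refresh the display.
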(event `self.ReceiveBeginPlay`
  (bind _aswb_texte_in_game (cast `/Game/UI_Widgets/WB_TexteInGame` (`self.GetWidget`) :!label _label))
  (bind _textblock_1 (`/Game/UI_Widgets/WB_TexteInGame.TextBlock_1` _aswb_texte_in_game))
  (`TextBlock.SetText` _textblock_1 (`self.AffichageTexte`))
  (bind (_font_fontobject _font_fontmaterial _font_outlinesettings _font_typefacefontname _font_size _font_letterspacing _font_skewamount _font_bforcemonospaced _font_monospacedwidth) (break `SlateFontInfo` (`TextBlock.Font` _textblock_1)))
  (`TextBlock.SetFont` _textblock_1 (make `SlateFontInfo` _font_fontobject _font_fontmaterial _font_outlinesettings _font_typefacefontname (`self.SizeText`) _font_letterspacing _font_skewamount _font_bforcemonospaced _font_monospacedwidth))
  (set `TextBlock.ColorAndOpacity` (make `SlateColor` (`self.ColorText`)) _textblock_1))

(event `UpdateWidget`
  (`KismetSystemLibrary.DelayUntilNextTick`)
  (goto _label))