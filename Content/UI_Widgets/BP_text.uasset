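; BP_text is a trigger actor that shows a tutorial text widget while the main third-person character is inside its box.
; The first overlap creates UI_textTuto through a DoOnce and adds it to the viewport.
; Later overlaps and exits find the first widget of that class by searching all widgets, then toggle it visible or hidden.
; Tick prints the cached character's movement direction to screen as debug output.
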(event `self.ReceiveBeginPlay`
  (bind _asbp_main_third_person_character (cast `/Game/Blueprints/Character/BP_MainThirdPersonCharacter` (`GameplayStatics.GetPlayerCharacter` 0)))
  (set `self.BP Main Third Person Character` _asbp_main_third_person_character))

(event `self.ReceiveTick`
  (params (DeltaSeconds :type "Float (single-precision)"))
  (bind _directionmouvement (`/Game/Blueprints/Character/BP_MainThirdPersonCharacter.DirectionMouvement` (`self.BP Main Third Person Character`)))
  (`KismetSystemLibrary.PrintString` (`KismetStringLibrary.Conv_IntToString` _directionmouvement) true false (struct :`R` 1.0 :`G` 0.083333 :`B` 0.947992 :`A` 1.0) 0.0)
  (if (!= _directionmouvement 0)
    _))

(event `self.Box.OnComponentBeginOverlap`
  (params (OverlappedComponent :type "PrimitiveComponent Object Reference") (OtherActor :type "Actor Object Reference") (OtherComp :type "PrimitiveComponent Object Reference") (OtherBodyIndex :type Integer) (bFromSweep :type Boolean) (SweepResult :type "HitResult Structure (by ref)"))
  (cast `/Game/Blueprints/Character/BP_MainThirdPersonCharacter` OtherActor)
  (`|ExecutionSequence`
    (:`then_0`
      (`/Engine/EditorBlueprintResources/StandardMacros.DoOnce` false
        (:`Completed`
          (bind _returnvalue (`|CreateWidget` "/Game/UI_Widgets/UI_Texte/UI_textTuto.UI_textTuto_C"))
          (`UserWidget.AddToViewport` _returnvalue 0))))
    (:`then_1`
      (`KismetSystemLibrary.PrintString` "in" true true (struct :`G` 0.041187 :`B` 1.0 :`A` 1.0))
      (bind _foundwidgets (`WidgetBlueprintLibrary.GetAllWidgetsOfClass` "/Game/UI_Widgets/UI_Texte/UI_textTuto.UI_textTuto_C" false))
      (bind _asui_text_tuto (cast `/Game/UI_Widgets/UI_Texte/UI_textTuto` (`|GetArrayItem` _foundwidgets)))
      (`Widget.SetVisibility` _asui_text_tuto "Visible"))))

(event `self.Box.OnComponentEndOverlap`
  (params (OverlappedComponent :type "PrimitiveComponent Object Reference") (OtherActor :type "Actor Object Reference") (OtherComp :type "PrimitiveComponent Object Reference") (OtherBodyIndex :type Integer))
  (cast `/Game/Blueprints/Character/BP_MainThirdPersonCharacter` OtherActor)
  (`KismetSystemLibrary.PrintString` "out" true true (struct :`R` 1.0 :`G` 0.242241 :`A` 1.0))
  (bind _foundwidgets (`WidgetBlueprintLibrary.GetAllWidgetsOfClass` "/Game/UI_Widgets/UI_Texte/UI_textTuto.UI_textTuto_C" false))
  (bind _asui_text_tuto (cast `/Game/UI_Widgets/UI_Texte/UI_textTuto` (`|GetArrayItem` _foundwidgets)))
  (`Widget.SetVisibility` _asui_text_tuto "Hidden"))

(fn `UserConstructionScript`)